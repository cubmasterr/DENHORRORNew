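; BP_Pickup_Gun_Vintares is an interactable Vintares gun pickup that a person can take as an item.
; On Interact, if the person's current item is not this gun, it disables collision on its six static mesh components.
; It then passes itself and its socket name to the person's PickUpItem, which handles the pickup.
; The construction script only calls the parent's.
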(event `/Game/Core/CharacterSystem/BPI_Interact.interact`
  (params (person :type "/Game/Core/CharacterSystem/BP_ThirdPersonCharacter Object Reference"))
  (if (!= (`/Game/Core/CharacterSystem/BP_ThirdPersonCharacter.item` person) self)
    (`PrimitiveComponent.SetCollisionEnabled` (`self.StaticMesh1`) "NoCollision")
    (`PrimitiveComponent.SetCollisionEnabled` (`self.StaticMesh2`) "NoCollision")
    (`PrimitiveComponent.SetCollisionEnabled` (`self.StaticMesh3`) "NoCollision")
    (`PrimitiveComponent.SetCollisionEnabled` (`self.StaticMesh4`) "NoCollision")
    (`PrimitiveComponent.SetCollisionEnabled` (`self.StaticMesh5`) "NoCollision")
    (`PrimitiveComponent.SetCollisionEnabled` (`self.StaticMesh`) "NoCollision")
    (`/Game/Core/CharacterSystem/BP_ThirdPersonCharacter.PickUpItem` person self (`self.SocetName`))))

(fn `UserConstructionScript`
  (`parent.UserConstructionScript`))