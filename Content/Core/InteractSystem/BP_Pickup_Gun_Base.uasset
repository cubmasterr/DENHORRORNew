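; BP_Pickup_Gun_Base is a base gun pickup that fires a hitscan shot for its owning BP_ThirdPersonCharacter.
; ShootGun line-traces on Visibility from the follow camera along its forward vector, adding random positive world Y/Z scatter to the end point.
; Hit actors implementing BPI_Hit receive Damage through HitMessage.
; Debug prints and trace drawing are active, and the construction script only calls the parent.
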(event `ShootGun`
  (bind _scattermax (`self.scatterMax`))
  (`KismetSystemLibrary.PrintString` "POOF")
  (bind _asbp_third_person_character (cast `/Game/Core/CharacterSystem/BP_ThirdPersonCharacter` (`self.GetOwner`)))
  (bind _followcamera (`/Game/Core/CharacterSystem/BP_ThirdPersonCharacter.FollowCamera` _asbp_third_person_character))
  (bind _returnvalue (`SceneComponent.K2_GetComponentLocation` _followcamera))
  (bind _outhit (`KismetSystemLibrary.LineTraceSingle` :`Start` _returnvalue :`End` (+ (+ _returnvalue (* (`SceneComponent.GetForwardVector` _followcamera) 100000.0)) (`KismetMathLibrary.MakeVector` 0.0 (`KismetMathLibrary.RandomFloatInRange` 0.0 _scattermax) (`KismetMathLibrary.RandomFloatInRange` 0.0 _scattermax))) :`TraceChannel` "TraceTypeQuery1" :`bTraceComplex` true :`DrawDebugType` "ForDuration"))
  (bind (_bblockinghit _binitialoverlap _time _distance _location _impactpoint _normal _impactnormal _physmat _hitactor) (`GameplayStatics.BreakHitResult` _outhit))
  (if (`KismetSystemLibrary.DoesImplementInterface` _hitactor "/Game/Core/HitObject/BPI_Hit.BPI_Hit_C")
    (message `/Game/Core/HitObject/BPI_Hit.Hit` _hitactor (`self.Damage`))
    (else
      (`KismetSystemLibrary.PrintString` "dont "))))

(fn `UserConstructionScript`
  (`parent.UserConstructionScript`))