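; Door actor in the interaction system that toggles open and closed each time its Action event fires.
; Action flips the Open0 flag, sets the target to either the Rotate value or zero rotation, then plays a timeline from the start.
; Each timeline update lerps the Scene component from its current relative rotation toward that target, so a re-trigger mid-swing reverses from where the door is.
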(event `self.action`
  (if (`self.Open_0`)
    (set `self.EndRotation` (struct))
    (set `self.Open_0` false)
    (bind (_direction _newtrack_0) (`Timeline|Timeline_0` :!via `PlayFromStart` :!label _label)
      (:`Update`
        (`SceneComponent.K2_SetRelativeRotation` (`self.Scene`) (`KismetMathLibrary.RLerp` (`SceneComponent.RelativeRotation` (`self.Scene`)) (`self.EndRotation`) _newtrack_0) false false)))
    (else
      (set `self.EndRotation` (`self.Rotate`))
      (set `self.Open_0` true)
      (goto _label :!via `PlayFromStart`))))

(fn `UserConstructionScript`
  (`parent.UserConstructionScript`))