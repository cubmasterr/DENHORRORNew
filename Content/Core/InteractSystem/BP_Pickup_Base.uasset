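; BP_Pickup_Base is a pickup actor in the interaction system, named as the base for items a person can pick up.
; On Interact, unless it is already that person's current Item, it disables its mesh collision and calls the person's PickUpItem with itself and a socket name.
; A separate ChaneItem function toggles the root component's visibility without propagating to children.
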(event `/Game/Core/CharacterSystem/BPI_Interact.interact`
  (params (person :type "/Game/Core/CharacterSystem/BP_ThirdPersonCharacter Object Reference"))
  (if (!= (`/Game/Core/CharacterSystem/BP_ThirdPersonCharacter.item` person) self)
    (`PrimitiveComponent.SetCollisionEnabled` (`self.Mesh`) "NoCollision")
    (`/Game/Core/CharacterSystem/BP_ThirdPersonCharacter.PickUpItem` person self (`self.SocetName`))))

(fn `ChaneItem`
  (`SceneComponent.ToggleVisibility` (`self.DefaultSceneRoot`) false))

(fn `UserConstructionScript`)